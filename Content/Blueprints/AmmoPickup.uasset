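; Ammo pickup actor that refills the player's weapons when anything overlaps its box while it is visible.
; It casts player 0's character and its nine weapon slots in a chain, setting each ammo count to a fixed amount; any failed cast stops the rest.
; A completed chain plays a sound and hides the pickup for a short delay, with the hidden state doubling as the cooldown.
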(event `self.Box1.OnComponentBeginOverlap`
  (params (OtherActor :type "Actor Object Reference") (OtherComp :type "PrimitiveComponent Object Reference") (OtherBodyIndex :type Integer) (bFromSweep :type Boolean) (SweepResult :type "EngineTypes.HitResult Structure (by ref)"))
  (if (not (`self.bHidden`))
    (bind _asmy_character (cast `/Game/Blueprints/MyCharacter` (`GameplayStatics.GetPlayerCharacter` 0)))
    (bind _aswp_pistol (cast `/Game/Blueprints/WP_Pistol` (`/Game/Blueprints/MyCharacter.weapon01` _asmy_character)))
    (set `/Game/Blueprints/WP_Pistol.AmmoCount` 100 _aswp_pistol)
    (bind _aswp_assault_rifle_retriggered (cast `/Game/Blueprints/WP_Assault_Rifle_Retriggered` (`/Game/Blueprints/MyCharacter.weapon02` _asmy_character)))
    (set `/Game/Blueprints/WP_Assault_Rifle_Retriggered.AmmoCount` 100 _aswp_assault_rifle_retriggered)
    (bind _aswp_assault_rifle_tail (cast `/Game/Blueprints/WP_Assault_Rifle_Tail` (`/Game/Blueprints/MyCharacter.weapon03` _asmy_character)))
    (set `/Game/Blueprints/WP_Assault_Rifle_Tail.AmmoCount` 100 _aswp_assault_rifle_tail)
    (bind _aswp_machine_gun (cast `/Game/Blueprints/WP_Machine_Gun` (`/Game/Blueprints/MyCharacter.weapon04` _asmy_character)))
    (set `/Game/Blueprints/WP_Machine_Gun.AmmoCount` 100 _aswp_machine_gun)
    (bind _aswp_sci_fi_beam (cast `/Game/Blueprints/WP_SciFi_Beam` (`/Game/Blueprints/MyCharacter.weapon05` _asmy_character)))
    (set `/Game/Blueprints/WP_SciFi_Beam.AmmoCount` 100 _aswp_sci_fi_beam)
    (bind _aswp_grenade_launcher (cast `/Game/Blueprints/WP_Grenade_Launcher` (`/Game/Blueprints/MyCharacter.weapon06` _asmy_character)))
    (set `/Game/Blueprints/WP_Grenade_Launcher.AmmoCount` 100 _aswp_grenade_launcher)
    (bind _aswp_assault_rifle_feedback (cast `/Game/Blueprints/WP_Assault_Rifle_Feedback` (`/Game/Blueprints/MyCharacter.weapon07` _asmy_character)))
    (set `/Game/Blueprints/WP_Assault_Rifle_Feedback.AmmoCount` 100 _aswp_assault_rifle_feedback)
    (bind _aswp_rifle (cast `/Game/Blueprints/WP_Rifle` (`/Game/Blueprints/MyCharacter.weapon08` _asmy_character)))
    (set `/Game/Blueprints/WP_Rifle.AmmoCount` 100 _aswp_rifle)
    (bind _aswp_assault_rifle_shells (cast `/Game/Blueprints/WP_Assault_Rifle_Shells` (`/Game/Blueprints/MyCharacter.weapon09` _asmy_character)))
    (set `/Game/Blueprints/WP_Assault_Rifle_Shells.AmmoCount` 100 _aswp_assault_rifle_shells)
    (`GameplayStatics.PlaySoundAttached` "/Engine/EditorSounds/Notifications/CompileSuccess.CompileSuccess" (`self.K2_GetRootComponent`))
    (`self.SetActorHiddenInGame` true)
    (`KismetSystemLibrary.Delay` 5.0)
    (`self.SetActorHiddenInGame` false)))

(fn `UserConstructionScript`)