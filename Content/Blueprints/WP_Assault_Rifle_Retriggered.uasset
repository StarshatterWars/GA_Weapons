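; Assault rifle weapon Blueprint that fires automatically while triggered, until released or out of ammo.
; Fire opens and enters a Gate, which re-enters itself after a short Delay for each shot; Release closes it.
; Each shot plays an attached sound, decrements AmmoCount and spawns a BasicUrbanProjectile at the offset muzzle socket, aimed along the player's control rotation.
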(event `Fire`
  (bind _returnvalue (`Pawn.GetControlRotation` (`GameplayStatics.GetPlayerPawn` 0)))
  (`|ExecutionSequence`
    (:`then_0`
      (goto _label :!via `Open`))
    (:`then_1`
      (`/Engine/EditorBlueprintResources/StandardMacros.Gate` true :!label _label
        (:`Exit`
          (if (> (`self.AmmoCount`) 0)
            (`GameplayStatics.PlaySoundAttached` "/Game/Audio/Assault_Rifle.Assault_Rifle" (`self.K2_GetRootComponent` (`GameplayStatics.GetPlayerCharacter` 0)))
            (set `self.AmmoCount` (- (`self.AmmoCount`) 1))
            (`|SpawnActorFromClass` "/Game/Blueprints/BasicUrbanProjectile.BasicUrbanProjectile_C" (`KismetMathLibrary.MakeTransform` (+ (`SceneComponent.GetSocketLocation` "MuzzleSocket") (`KismetMathLibrary.GreaterGreater_VectorRotator` (`self.GunOffset`) _returnvalue)) _returnvalue) true)
            (`KismetSystemLibrary.Delay` 0.1)
            (goto _label)))))))

(event `Release`
  (goto _label :!via `Close`))

(fn `UserConstructionScript`)