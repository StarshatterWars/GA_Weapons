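; Grenade launcher weapon Blueprint that fires grenade projectiles from a limited ammo count.
; The Fire event checks ammo, plays an attached shot sound, decrements the count and spawns GrenadeProj even if colliding.
; Spawn location is the weapon's position plus a rotated gun offset, with aim taken from player 0's control rotation.
; A DoOnce reset after a short delay limits the fire rate.
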(event `Fire`
  (bind _returnvalue (`Pawn.GetControlRotation` (`GameplayStatics.GetPlayerPawn` 0)))
  (if (> (`self.AmmoCount`) 0)
    (`/Engine/EditorBlueprintResources/StandardMacros.DoOnce` false :!label _label
      (:`Completed`
        (`GameplayStatics.PlaySoundAttached` "/Game/Audio/GrenadeLauncher_Shot_Cue.GrenadeLauncher_Shot_Cue" (`self.SkeletalMesh1`) "None" (0.0 0.0 0.0) "SnapToTarget")
        (set `self.AmmoCount` (- (`self.AmmoCount`) 1))
        (`|SpawnActorFromClass` "/Game/Blueprints/GrenadeProj.GrenadeProj_C" (`KismetMathLibrary.MakeTransform` (+ (`self.K2_GetActorLocation`) (`KismetMathLibrary.GreaterGreater_VectorRotator` (`self.GunOffset`) _returnvalue)) _returnvalue) true)
        (`KismetSystemLibrary.Delay` 0.5)
        (goto _label :!via `Reset`)))))

(fn `UserConstructionScript`)