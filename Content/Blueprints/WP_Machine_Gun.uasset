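; Machine gun weapon Blueprint that fires automatically between its Fire and Release events while ammo remains.
; Fire starts an attached looping sound and opens a Gate, which a short Delay re-enters to repeat shots.
; Each shot decrements AmmoCount and spawns a BasicUrbanProjectile at the offset muzzle socket, aimed along player 0's control rotation.
; Release or empty ammo closes the Gate, stops the loop and plays a tail sound.
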(event `Fire`
  (bind _returnvalue (`self.K2_GetRootComponent`))
  (bind _returnvalue_2 (> (`self.AmmoCount`) 0))
  (bind _returnvalue_3 (`Pawn.GetControlRotation` (`GameplayStatics.GetPlayerPawn` 0)))
  (if _returnvalue_2
    (`|ExecutionSequence`
      (:`then_0`
        (bind _returnvalue_4 (`GameplayStatics.PlaySoundAttached` "/Game/Audio/Machine_Gun_Loop.Machine_Gun_Loop" _returnvalue)))
      (:`then_1`
        (goto _label :!via `Open`))
      (:`then_2`
        (`/Engine/EditorBlueprintResources/StandardMacros.Gate` true :!label _label
          (:`Exit`
            (if _returnvalue_2
              (set `self.AmmoCount` (- (`self.AmmoCount`) 1))
              (`|SpawnActorFromClass` "/Game/Blueprints/BasicUrbanProjectile.BasicUrbanProjectile_C" (`KismetMathLibrary.MakeTransform` (+ (`SceneComponent.GetSocketLocation` "MuzzleSocket") (`KismetMathLibrary.GreaterGreater_VectorRotator` (`self.GunOffset`) _returnvalue_3)) _returnvalue_3) true)
              (`KismetSystemLibrary.Delay` 0.05)
              (goto _label)
              (else
                (`|ExecutionSequence`
                  (:`then_0`
                    (goto _label :!via `Close`))
                  (:`then_1`
                    (`AudioComponent.Stop` _returnvalue_4 :!label _label_2))
                  (:`then_2`
                    (`GameplayStatics.PlaySoundAttached` "/Game/Audio/Machine_Gun_Tail.Machine_Gun_Tail" _returnvalue :!label _label_3)))))))))))

(event `Release`
  (if (> (`self.AmmoCount`) 0)
    (`|ExecutionSequence`
      (:`then_0`
        (goto _label :!via `Close`))
      (:`then_1`
        (goto _label_2))
      (:`then_2`
        (goto _label_3)))))

(fn `UserConstructionScript`)