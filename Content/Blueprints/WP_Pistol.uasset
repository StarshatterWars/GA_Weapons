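; WP_Pistol is a pistol weapon Blueprint that fires projectiles for the player while it has ammo.
; Its Fire event plays an attached pistol sound, decrements AmmoCount and spawns a BasicUrbanProjectile from the MuzzleSocket, offset by GunOffset along the player's control rotation.
; A DoOnce reset after a short Delay limits the rate of fire.
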(event `Fire`
  (bind _returnvalue (`Pawn.GetControlRotation` (`GameplayStatics.GetPlayerPawn` 0)))
  (if (> (`self.AmmoCount`) 0)
    (`/Engine/EditorBlueprintResources/StandardMacros.DoOnce` false :!label _label
      (:`Completed`
        (`GameplayStatics.PlaySoundAttached` "/Game/Audio/Pistol.Pistol" (`self.K2_GetRootComponent` (`GameplayStatics.GetPlayerCharacter` 0)))
        (set `self.AmmoCount` (- (`self.AmmoCount`) 1))
        (`|SpawnActorFromClass` "/Game/Blueprints/BasicUrbanProjectile.BasicUrbanProjectile_C" (`KismetMathLibrary.MakeTransform` (+ (`SceneComponent.GetSocketLocation` "MuzzleSocket") (`KismetMathLibrary.GreaterGreater_VectorRotator` (`self.GunOffset`) _returnvalue)) _returnvalue) true)
        (`KismetSystemLibrary.Delay` 0.5)
        (goto _label :!via `Reset`)))))

(fn `UserConstructionScript`)