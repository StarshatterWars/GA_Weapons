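; Rifle weapon Blueprint that fires projectiles with gunshot tails matched to the acoustic space around it.
; Fire checks ammo, spawns BasicUrbanProjectile from the muzzle along the player's control rotation, and uses a delayed DoOnce reset to limit fire rate.
; A box overlap finds the highest-priority GAB_WeaponTailsVolume, whose name selects the tail through the WaveSelect parameter, layered over the dry shot sound.
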(event `Fire`
  (bind _returnvalue (`self.K2_GetRootComponent`))
  (bind _weapontailsvolumenamearray (`self.WeaponTailsVolumeNameArray`))
  (bind _weapontailsvolumepriorityarray (`self.WeaponTailsVolumePriorityArray`))
  (bind _returnvalue_2 (`Pawn.GetControlRotation` (`GameplayStatics.GetPlayerPawn` 0)))
  (bind _item (`KismetArrayLibrary.Array_Get` _weapontailsvolumenamearray (`KismetMathLibrary.MaxOfIntArray` _weapontailsvolumepriorityarray)))
  (if (> (`self.AmmoCount`) 0)
    (`/Engine/EditorBlueprintResources/StandardMacros.DoOnce` false :!label _label
      (:`Completed`
        (`KismetArrayLibrary.Array_Clear` (`self.WeaponTailsVolumeNameArray`))
        (`KismetArrayLibrary.Array_Clear` (`self.WeaponTailsVolumePriorityArray`))
        (bind _outactors (`KismetSystemLibrary.BoxOverlapActors_NEW` (`self.K2_GetActorLocation`) (5.0 5.0 5.0) (`|MakeArray` "ObjectTypeQuery2" :!type "EngineTypes.EObjectTypeQuery Enum")))
        (for _array_element _outactors
          (bind _asgab_weapon_tails_volume (cast `/Game/Blueprints/GAB_WeaponTailsVolume` _array_element))
          (`KismetArrayLibrary.Array_Add` _weapontailsvolumenamearray (`/Game/Blueprints/GAB_WeaponTailsVolume.VolumeName` _asgab_weapon_tails_volume))
          (`KismetArrayLibrary.Array_Add` _weapontailsvolumepriorityarray (`/Game/Blueprints/GAB_WeaponTailsVolume.Priority` _asgab_weapon_tails_volume)))
        (`GameplayStatics.PlaySoundAttached` "/Game/Audio/Rifle_Dry_Cue.Rifle_Dry_Cue" _returnvalue)
        (if (`KismetStringLibrary.EqualEqual_StrStr` _item "SmallRoom")
          (set `self.ReverbTails` 0)
          (bind _returnvalue_3 (`GameplayStatics.PlaySoundAttached` "/Game/Audio/UrbanRifleTails.UrbanRifleTails" _returnvalue :!label _label_2))
          (`AudioComponent.SetIntParameter` _returnvalue_3 "WaveSelect" (`self.ReverbTails`))
          (set `self.AmmoCount` (- (`self.AmmoCount`) 1))
          (`|SpawnActorFromClass` "/Game/Blueprints/BasicUrbanProjectile.BasicUrbanProjectile_C" (`KismetMathLibrary.MakeTransform` (+ (`SceneComponent.GetSocketLocation` "MuzzleSocket") (`KismetMathLibrary.GreaterGreater_VectorRotator` (`self.GunOffset`) _returnvalue_2)) _returnvalue_2) true)
          (`KismetSystemLibrary.Delay` 0.5)
          (goto _label :!via `Reset`)
          (elif (`KismetStringLibrary.EqualEqual_StrStr` _item "LargeRoom")
            (set `self.ReverbTails` 1)
            (goto _label_2)
            (elif (`KismetStringLibrary.EqualEqual_StrStr` _item "Street")
              (set `self.ReverbTails` 2)
              (goto _label_2)
              (elif (`KismetStringLibrary.EqualEqual_StrStr` _item "Outside")
                (set `self.ReverbTails` 3)
                (goto _label_2)))))))))

(fn `UserConstructionScript`)