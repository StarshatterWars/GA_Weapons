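; Assault rifle weapon Blueprint with automatic fire, ammo consumption and a separate tail sound when firing stops.
; Fire opens a Gate that loops through a short Delay, each pass playing a shot sound and spawning a BasicUrbanProjectile from MuzzleSocket along the player's control rotation.
; Release closes the Gate and plays the tail if ammo remains; the loop plays it when ammo runs out.
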(event `Fire`
  (bind _returnvalue (`self.K2_GetRootComponent`))
  (bind _returnvalue_2 (> (`self.AmmoCount`) 0))
  (bind _returnvalue_3 (`Pawn.GetControlRotation` (`GameplayStatics.GetPlayerPawn` 0)))
  (if _returnvalue_2
    (`|ExecutionSequence`
      (:`then_0`
        (goto _label :!via `Open`))
      (:`then_1`
        (`/Engine/EditorBlueprintResources/StandardMacros.Gate` true :!label _label
          (:`Exit`
            (if _returnvalue_2
              (`GameplayStatics.PlaySoundAttached` "/Game/Audio/Assault_Rifle_Shot.Assault_Rifle_Shot" _returnvalue)
              (set `self.AmmoCount` (- (`self.AmmoCount`) 1))
              (`|SpawnActorFromClass` "/Game/Blueprints/BasicUrbanProjectile.BasicUrbanProjectile_C" (`KismetMathLibrary.MakeTransform` (+ (`SceneComponent.GetSocketLocation` "MuzzleSocket") (`KismetMathLibrary.GreaterGreater_VectorRotator` (`self.GunOffset`) _returnvalue_3)) _returnvalue_3) true)
              (`KismetSystemLibrary.Delay` 0.075)
              (goto _label)
              (else
                (`GameplayStatics.PlaySoundAttached` "/Game/Audio/Assault_Rifle_Tail.Assault_Rifle_Tail" _returnvalue :!label _label_2)))))))))

(event `Release`
  (if (> (`self.AmmoCount`) 0)
    (`|ExecutionSequence`
      (:`then_0`
        (goto _label :!via `Close`))
      (:`then_1`
        (goto _label_2)))))

(fn `UserConstructionScript`)