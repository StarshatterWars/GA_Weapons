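; Assault rifle weapon Blueprint that fires projectiles automatically and gives audio feedback when ammo runs low.
; Fire opens a Gate and shoots at once, then a short Delay re-enters the Gate to repeat until Release closes it or ammo runs out.
; Each shot picks the normal or low-ammo sound, decrements ammo, and spawns a BasicUrbanProjectile offset from the muzzle socket along the first player's control rotation.
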(event `Fire`
  (bind _returnvalue (`self.K2_GetRootComponent`))
  (bind _returnvalue_2 (`Pawn.GetControlRotation` (`GameplayStatics.GetPlayerPawn` 0)))
  (if (> (`self.AmmoCount`) 0)
    (`|ExecutionSequence`
      (:`then_0`
        (goto _label_2 :!via `Open`))
      (:`then_1`
        (if (> (`self.AmmoCount`) 20) :!label _label
          (`GameplayStatics.PlaySoundAttached` "/Game/Audio/Assault_Rifle.Assault_Rifle" _returnvalue)
          (else
            (`GameplayStatics.PlaySoundAttached` "/Game/Audio/WEAPON_FeedbackMech_LowAmmo_Cue.WEAPON_FeedbackMech_LowAmmo_Cue" _returnvalue)))
        (set `self.AmmoCount` (- (`self.AmmoCount`) 1))
        (`|SpawnActorFromClass` "/Game/Blueprints/BasicUrbanProjectile.BasicUrbanProjectile_C" (`KismetMathLibrary.MakeTransform` (+ (`SceneComponent.GetSocketLocation` "MuzzleSocket") (`KismetMathLibrary.GreaterGreater_VectorRotator` (`self.GunOffset`) _returnvalue_2)) _returnvalue_2) true)
        (`KismetSystemLibrary.Delay` 0.1)
        (if (> (`self.AmmoCount`) 0)
          (`/Engine/EditorBlueprintResources/StandardMacros.Gate` true :!label _label_2
            (:`Exit`
              (goto _label))))))))

(event `Release`
  (goto _label_2 :!via `Close`))

(fn `UserConstructionScript`)