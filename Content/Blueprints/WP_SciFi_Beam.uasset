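; Sci-fi beam weapon that fires continuously from Fire until Release or until its ammo runs out.
; Fire plays a start sound, then attaches a looping sound and a beam particle to the muzzle socket.
; A Gate and Delay loop drains one ammo per tick while firing.
; Release or empty ammo closes the gate, plays a stop sound, and removes the loop sound and particle.
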(event `Fire`
  (bind _returnvalue (`self.K2_GetRootComponent`))
  (bind _returnvalue_2 (> (`self.AmmoCount`) 0))
  (if _returnvalue_2
    (`|ExecutionSequence`
      (:`then_0`
        (goto _label_2 :!via `Open`))
      (:`then_1`
        (`KismetSystemLibrary.Delay` 0.2 :!label _label)
        (set `self.AmmoCount` (- (`self.AmmoCount`) 1))
        (if _returnvalue_2
          (`/Engine/EditorBlueprintResources/StandardMacros.Gate` true :!label _label_2
            (:`Exit`
              (goto _label)))
          (else
            (`|ExecutionSequence`
              (:`then_0`
                (goto _label_2 :!via `Close`))
              (:`then_1`
                (`GameplayStatics.SpawnSoundAttached` "/Game/Audio/BeamStop.BeamStop" _returnvalue :!label _label_3)
                (`AudioComponent.Stop` (stale _returnvalue_3))
                (`ActorComponent.K2_DestroyComponent` (stale _returnvalue_4)))))))
      (:`then_2`
        (`GameplayStatics.SpawnSoundAttached` "/Game/Audio/BeamStart.BeamStart" _returnvalue)
        (bind _returnvalue_3 (`GameplayStatics.SpawnSoundAttached` "/Game/Audio/BeamLoop.BeamLoop" _returnvalue))
        (bind _returnvalue_4 (`GameplayStatics.SpawnEmitterAttached` "/Game/Weapon_Assets/Beam/P_Beam.P_Beam" (`self.SkeletalMesh1`) "MuzzleSocket" (0.0 0.0 0.0) (struct :`Pitch` 90.0)))))))

(event `Release`
  (if (> (`self.AmmoCount`) 0)
    (`|ExecutionSequence`
      (:`then_0`
        (goto _label_2 :!via `Close`))
      (:`then_1`
        (goto _label_3)))))

(fn `UserConstructionScript`)