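; Assault rifle weapon Blueprint that fires projectiles automatically while the trigger is held, with shell casing sounds that match the ground surface.
; Fire opens a Gate that loops on a short Delay, using up ammo and spawning a projectile from the muzzle socket along the player's control rotation.
; A downward trace each shot picks concrete or metal casing audio by physical material.
; Release or running dry plays the tail sound.
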(event `Fire`
  (bind _returnvalue (`self.K2_GetRootComponent`))
  (bind _returnvalue_2 (`self.K2_GetActorLocation`))
  (bind _returnvalue_3 (`self.K2_GetRootComponent`))
  (bind _returnvalue_4 (> (`self.AmmoCount`) 0))
  (bind _returnvalue_5 (`Pawn.GetControlRotation` (`GameplayStatics.GetPlayerPawn` 0)))
  (if _returnvalue_4
    (`|ExecutionSequence`
      (:`then_0`
        (goto _label :!via `Open`))
      (:`then_1`
        (`/Engine/EditorBlueprintResources/StandardMacros.Gate` true :!label _label
          (:`Exit`
            (if _returnvalue_4
              (`GameplayStatics.PlaySoundAttached` "/Game/Audio/Assault_Rifle_Shot.Assault_Rifle_Shot" _returnvalue_3)
              (set `self.AmmoCount` (- (`self.AmmoCount`) 1))
              (`|SpawnActorFromClass` "/Game/Blueprints/ImpactProjectile.ImpactProjectile_C" (`KismetMathLibrary.MakeTransform` (+ (`SceneComponent.GetSocketLocation` "MuzzleSocket") (`KismetMathLibrary.GreaterGreater_VectorRotator` (`self.GunOffset`) _returnvalue_5)) _returnvalue_5) true)
              (bind _outhit (`KismetSystemLibrary.LineTraceSingle` _returnvalue_2 (- _returnvalue_2 (0.0 0.0 200.0)) "TraceTypeQuery1"))
              (switch `EngineTypes.EPhysicalSurface` (`PhysicalMaterial.SurfaceType` (`.PhysMat` (`GameplayStatics.BreakHitResult` _outhit)))
                (:`SurfaceType_Default`
                  _)
                (:`SurfaceType1`
                  (`GameplayStatics.PlaySoundAttached` "/Game/Audio/ShellCasings_Concrete.ShellCasings_Concrete" _returnvalue))
                (:`SurfaceType2`
                  (`GameplayStatics.PlaySoundAttached` "/Game/Audio/ShellCasings_Metal.ShellCasings_Metal" _returnvalue)))
              (`KismetSystemLibrary.Delay` 0.1)
              (goto _label)
              (else
                (`GameplayStatics.PlaySoundAttached` "/Game/Audio/Assault_Rifle_Tail.Assault_Rifle_Tail" _returnvalue_3 :!label _label_2)))))))))

(event `Release`
  (if (> (`self.AmmoCount`) 0)
    (`|ExecutionSequence`
      (:`then_0`
        (goto _label :!via `Close`))
      (:`then_1`
        (goto _label_2)))))

(fn `UserConstructionScript`)